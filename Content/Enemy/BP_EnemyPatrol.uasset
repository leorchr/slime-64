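; BP_EnemyPatrol is an enemy character that chases the player inside a detection sphere; its Patrol event is still empty.
; Overlaps with a Player-tagged root component toggle PlayerSpot, and BeginPlay applies the speed and detection radius.
; While spotted, Tick updates the destination to the player's location and calls AIMoveTo each frame.
; Once lost, movement is disabled upon reaching the last known position; Tick also draws a debug sphere.
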(event `Patrol`
  ;[0.04179 1 0] Patrol
)

(event `Follow Player`
  ;[1 0 0.7934] Go to player position
  (if (`self.PlayerSpot`)
    (`|AIMoveTo` self (`self.ObjectifDestination`) null (`self.Distance Destination`))))

(event `self.ReceiveTick`
  (params (DeltaSeconds :type "Float (single-precision)"))
  ;[1 1 1] Debug
  (`KismetSystemLibrary.DrawDebugSphere` (`self.K2_GetActorLocation` self) (`self.Detection Size`) 12 (struct :`R` 1.0 :`G` 0.008092 :`A` 1.0) 0.1 1.0)
  ;[0.3312 1 0.4138] Get Player Position
  (if (`self.PlayerSpot`)
    (set `self.ObjectifDestination` (`self.K2_GetActorLocation` (cast `/Game/ThirdPerson/Blueprints/BP_ThirdPersonCharacter` (`GameplayStatics.GetPlayerCharacter` 0) :!pure true)))
    (`CharacterMovementComponent.SetMovementMode` (`self.CharacterMovement`) "MOVE_Walking" 0)
    (`self.Follow Player`)
    (else
      (`self.Stop Follow Player`))))

(event `Stop Follow Player`
  ;[1 0 0] Stop Follow
  (if (`self.PlayerSpot`)
    _
    (elif (== (`self.K2_GetActorLocation` self) (`self.ObjectifDestination`) :`ErrorTolerance` 15.0)
      (`CharacterMovementComponent.SetMovementMode` (`self.CharacterMovement`) "MOVE_None" 0))))

(event `self.ReceiveBeginPlay`
  ;[0 1 0.2663] Set Variables
  (set `CharacterMovementComponent.MaxWalkSpeed` (`self.Enemy Speed`) (`self.CharacterMovement`))
  (`SphereComponent.SetSphereRadius` (`self.Detection Player Sphere`) (`self.Detection Size`) true))

(event `self.Detection Player Sphere.OnComponentBeginOverlap`
  (params (OverlappedComponent :type "PrimitiveComponent Object Reference") (OtherActor :type "Actor Object Reference") (OtherComp :type "PrimitiveComponent Object Reference") (OtherBodyIndex :type Integer) (bFromSweep :type Boolean) (SweepResult :type "HitResult Structure (by ref)"))
  ;[0 1 0.991] All Overlap
  (if (`ActorComponent.ComponentHasTag` (`Actor.RootComponent` OtherActor) "Player")
    (bind _output_get (set `self.PlayerSpot` true))
    (`KismetSystemLibrary.PrintString` (`KismetStringLibrary.Conv_BoolToString` _output_get))))

(event `self.Detection Player Sphere.OnComponentEndOverlap`
  (params (OverlappedComponent :type "PrimitiveComponent Object Reference") (OtherActor :type "Actor Object Reference") (OtherComp :type "PrimitiveComponent Object Reference") (OtherBodyIndex :type Integer))
  ;[0 1 0.991] All Overlap
  (if (`ActorComponent.ComponentHasTag` (`Actor.RootComponent` OtherActor) "Player")
    (bind _output_get (set `self.PlayerSpot` false))
    (`KismetSystemLibrary.PrintString` (`KismetStringLibrary.Conv_BoolToString` _output_get))))

(fn `UserConstructionScript`)