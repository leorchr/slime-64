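; Grindable rail for the platformer system that builds its mesh along a spline and plays a grinding sound while in use.
; The construction script tiles spline mesh sections of a set length along the spline, clamping tangents to that length and enabling collision.
; At BeginPlay, unless it is a child actor, it creates an audio component and binds the OnEnter and OnExit events that start and stop the sound.
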(event `self.ReceiveBeginPlay`
  (if (not (`self.IsChildActor`))
    (add `self.OnEnter` (delegate `OnEnter_Event`))
    (add `self.OnExit` (delegate `OnExit_Event`))
    (bind _returnvalue (`AddComponent|NODE_AddAudioComponent-0`))
    (set `self.RailGrinding_Audio` _returnvalue)))

(event `OnEnter_Event`
  (`AudioComponent.SetSound` (`self.RailGrinding_Audio`) "/Game/04_Sounds/SFX/Rail/A_RailGrinding.A_RailGrinding")
  (`AudioComponent.Play` (`self.RailGrinding_Audio`) 0.0))

(event `OnExit_Event`
  (`AudioComponent.Stop` (`self.RailGrinding_Audio`)))

(fn `UserConstructionScript`
  (bind _splinecomponent (`self.SplineComponent`))
  (bind _splinecomponent_2 (`self.SplineComponent`))
  (bind _sectionlength (`self.SectionLength`))
  (bind _sectionlength_2 (`self.SectionLength`))
  (for _index (range (+ (`KismetMathLibrary.FTrunc` (/ (`SplineComponent.GetSplineLength` (`self.SplineComponent`)) (`self.SectionLength`))) 1))
    (bind _returnvalue (`AddComponent|NODE_AddSplineMeshComponent-1`))
    (`StaticMeshComponent.SetStaticMesh` _returnvalue (`self.Mesh`))
    (`SplineMeshComponent.SetForwardAxis` _returnvalue "Z" true)
    (`SceneComponent.SetWorldScale3D` _splinecomponent (`self.MeshScale`))
    (bind _returnvalue_2 (* _index _sectionlength_2))
    (bind _returnvalue_3 (* (+ _index 1) _sectionlength))
    (`SplineMeshComponent.SetStartAndEnd` _returnvalue (`SplineComponent.GetLocationAtDistanceAlongSpline` _splinecomponent _returnvalue_2 "Local") (`KismetMathLibrary.ClampVectorSize` (`SplineComponent.GetTangentAtDistanceAlongSpline` _splinecomponent _returnvalue_2 "Local") 0.0 _sectionlength_2) (`SplineComponent.GetLocationAtDistanceAlongSpline` _splinecomponent_2 _returnvalue_3 "Local") (`KismetMathLibrary.ClampVectorSize` (`SplineComponent.GetTangentAtDistanceAlongSpline` _splinecomponent_2 _returnvalue_3 "Local") 0.0 _sectionlength) true)
    (`PrimitiveComponent.SetCollisionEnabled` _returnvalue "QueryAndPhysics")
    (`PrimitiveComponent.SetCollisionEnabled` _returnvalue "QueryAndPhysics")))