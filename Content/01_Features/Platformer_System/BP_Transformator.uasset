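; BP_Transformator is a platformer machine that switches the player character's Blob mesh between cube and sphere.
; Box overlap by a BP_Character disables input, snaps the character to the box and zeroes its velocity.
; Tick lowers the Mold with a clamped lerp, swaps the mesh at the bottom, then raises it and restores input.
; The IsCube toggle lives on the machine, not the character.
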(event `self.Box.OnComponentBeginOverlap`
  (params (OverlappedComponent :type "PrimitiveComponent Object Reference") (OtherActor :type "Actor Object Reference") (OtherComp :type "PrimitiveComponent Object Reference") (OtherBodyIndex :type Integer) (bFromSweep :type Boolean) (SweepResult :type "HitResult Structure (by ref)"))
  (if (not (`self.isTransformating`))
    (bind _asbp_character (cast `/Game/00_GameManager/Character/BP_Character` OtherActor))
    (`self.StopPlayer` _asbp_character)
    (set `self.ForwardDir` true)
    (set `self.isTransformating` true)
    (set `self.currentCharacter` _asbp_character)))

(event `self.ReceiveTick`
  (params (DeltaSeconds :type "Float (single-precision)"))
  (if (`self.isTransformating`)
    (if (`self.ForwardDir`)
      (bind _output_get (set `self.moveT` (`KismetMathLibrary.FClamp` (+ (`self.moveT`) (* DeltaSeconds (`self.Speed`))))))
      (`SceneComponent.K2_SetRelativeLocation` (`self.Mold`) (`KismetMathLibrary.MakeVector` 0.0 0.0 (`KismetMathLibrary.Lerp` 160.0 60.0 _output_get)) false false)
      (if (== (`self.moveT`) 1.0)
        (set `self.ForwardDir` false)
        (`self.Transform` (`self.currentCharacter`)))
      (else
        (bind _output_get_2 (set `self.moveT` (`KismetMathLibrary.FClamp` (- (`self.moveT`) (* DeltaSeconds (`self.Speed`))))))
        (`SceneComponent.K2_SetRelativeLocation` (`self.Mold`) (`KismetMathLibrary.MakeVector` 0.0 0.0 (`KismetMathLibrary.Lerp` 160.0 60.0 _output_get_2)) false false)
        (if (== (`self.moveT`) 0.0)
          (set `self.ForwardDir` false)
          (set `self.isTransformating` false)
          (`self.MovePlayer`))))))

(event `self.Box.OnComponentEndOverlap`
  (params (OverlappedComponent :type "PrimitiveComponent Object Reference") (OtherActor :type "Actor Object Reference") (OtherComp :type "PrimitiveComponent Object Reference") (OtherBodyIndex :type Integer)))

(fn `MovePlayer`
  (bind _asbp_controller (cast `/Game/00_GameManager/Controller/BP_Controller` (`Pawn.GetController` (`self.currentCharacter`))))
  (`self.EnableInput` _asbp_controller _asbp_controller))

(fn `StopPlayer`
  (params (Character :type "/Game/00_GameManager/Character/BP_Character Object Reference"))
  (bind _returnvalue (`Pawn.GetController` Character))
  (bind _asbp_controller (cast `/Game/00_GameManager/Controller/BP_Controller` _returnvalue))
  (`self.DisableInput` _returnvalue _asbp_controller)
  (`self.K2_SetActorLocation` Character (`SceneComponent.K2_GetComponentLocation` (`self.Box`)) false false)
  (set `MovementComponent.Velocity` (0.0 0.0 0.0) (`Character.CharacterMovement` Character)))

(fn `Transform`
  (params (Character :type "/Game/00_GameManager/Character/BP_Character Object Reference"))
  (`StaticMeshComponent.SetStaticMesh` (`/Game/00_GameManager/Character/BP_Character.Blob` Character) (select `bool` (`self.isCube`) :`false` (`self.CubeMesh`) :`true` (`self.SphereMesh`)))
  (set `self.isCube` (not (`self.isCube`))))

(fn `UserConstructionScript`)