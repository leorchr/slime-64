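; Platformer cannon actor that gives audio, visual and UI feedback as something enters and leaves its child BP_Rail.
; It binds to the rail's enter and exit events on BeginPlay and caches the cannon mesh's base scale.
; Entering plays a sound and a timeline that scales up the mesh, with a DoOnce adding the prompt widget.
; Exiting plays the shot sound and smoke, removes the prompt and resets the DoOnce.
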(event `self.ReceiveBeginPlay`
  (bind _asbp_rail (cast `/Game/01_Features/Platformer_System/BP_Rail` (`ChildActorComponent.ChildActor` (`self.BP_Rail`))))
  (add `Rail.OnEnter` _asbp_rail (delegate `On Enter Rail`))
  (add `Rail.OnExit` _asbp_rail (delegate `OnExitRail`))
  (set `self.BaseScale` (`SceneComponent.RelativeScale3D` (`self.SM_M_Canon`))))

(event `On Enter Rail`
  (`GameplayStatics.PlaySoundAtLocation` "/Game/04_Sounds/SFX/Cannon/A_CannonEntering.A_CannonEntering" (`self.K2_GetActorLocation`) (struct) 1.0 1.0 0.0 null null null null)
  (bind (_direction _alpha) (`Timeline|Entering` :!via `PlayFromStart`)
    (:`Update`
      (`SceneComponent.SetRelativeScale3D` (`self.SM_M_Canon`) (`KismetMathLibrary.VLerp` (`self.BaseScale`) (1.5 1.5 1.5) _alpha))
      (`/Engine/EditorBlueprintResources/StandardMacros.DoOnce` false :!label _label
        (:`Completed`
          (bind _returnvalue (`|CreateWidget` "/Game/03_UI/WBP/WBP_PromptCanon.WBP_PromptCanon_C"))
          (bind _output_get (set `self.UI_Prompt` _returnvalue))
          (`UserWidget.AddToViewport` _output_get 0))))))

(event `OnExitRail`
  (`GameplayStatics.PlaySoundAtLocation` "/Game/04_Sounds/SFX/Cannon/A_CannonShoot.A_CannonShoot" (`self.K2_GetActorLocation`) (struct) 1.0 1.0 0.0 null null null null)
  (`ActorComponent.Activate` (`self.ShootSmoke`) false)
  (`Widget.RemoveFromParent` (`self.UI_Prompt`))
  (goto _label :!via `Reset`))

(fn `UserConstructionScript`)