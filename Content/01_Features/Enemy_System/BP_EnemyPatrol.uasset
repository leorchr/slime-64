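; Patrolling enemy that dashes at the player on sight and dies after enough hits from player overlaps.
; It walks to random navmesh points around its spawn, with Tick picking new ones on arrival or when stationary.
; PawnSensing triggers a launch and move to the player's seen position, then a stun with Niagara VFX.
; HurtBox overlaps remove HP with a cooldown, and debug spheres show sight and patrol ranges.
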(event `self.PawnSensing.OnSeePawn`
  (params (Pawn :type "Pawn Object Reference"))
  (bind _niagara (`self.Niagara`))
  ;[1 0.5979 0.7089] Go to player position
  (if (== Pawn (`GameplayStatics.GetPlayerCharacter` 0))
    (set `self.PlayerSpot` true)
    (`SceneComponent.SetHiddenInGame` (`self.Widget`) false false)
    (bind _output_get (set `self.ObjectifDestination` (`self.K2_GetActorLocation` Pawn)))
    (set `CharacterMovementComponent.MaxWalkSpeed` (`self.Dash Speed`) (`self.CharacterMovement`))
    (`/Engine/EditorBlueprintResources/StandardMacros.DoOnce` false :!label _label
      (:`Completed`
        (`self.LaunchCharacter` (* (`KismetMathLibrary.GetForwardVector` (`self.K2_GetActorRotation`)) (`self.Dash Speed`)))
        (`|AIMoveTo` self _output_get null (`self.Acceptance Distance Player`)
          (:`OnSuccess`
            (`self.Dsh Reset`))
          (:`OnFail`
            (`self.Dsh Reset`)))
        (`ActorComponent.Activate` _niagara false)
        (set `CharacterMovementComponent.MaxWalkSpeed` 0.0 (`self.CharacterMovement`))
        (`KismetSystemLibrary.Delay` (`self.StunDuration`))
        (set `self.PlayerSpot` false)
        (set `CharacterMovementComponent.MaxWalkSpeed` (`self.Enemy Speed`) (`self.CharacterMovement`))
        (`ActorComponent.Deactivate` _niagara)))
    (else
      (set `self.PlayerSpot` false))))

(event `Dsh Reset`
  ;[1 0.5979 0.7089] Go to player position
  (goto _label :!via `Reset`))

(event `Stop Follow Player`
  ;[1 0 0] Stop Follow
  (if (`self.PlayerSpot`)
    _
    (elif (== (`self.K2_GetActorLocation`) (`self.ObjectifDestination`) :`ErrorTolerance` 100.0)
      (`self.Patrol`))))

(event `self.ReceiveTick`
  (params (DeltaSeconds :type "Float (single-precision)"))
  ;[1 1 1] Debug
  (`KismetSystemLibrary.DrawDebugSphere` (`self.K2_GetActorLocation` self) (`self.Detection Size`) 12 (struct :`R` 1.0 :`G` 0.008092 :`A` 1.0) 0.1 1.0)
  (`KismetSystemLibrary.DrawDebugSphere` (`self.Origin Enemy Patrol`) (`self.Range Patrol Enemy`) 12 (struct :`G` 1.0 :`B` 1.0 :`A` 1.0) 0.1 1.0)
  ;[0.3312 1 0.4138] Get Player Position
  (if (not (`self.PlayerSpot`))
    (`self.Stop Follow Player`)
    (`KismetSystemLibrary.Delay` 2.0)
    (if (== (`KismetMathLibrary.VSize` (`self.GetVelocity`)) 0.0)
      (bind _output_get (set `self.Stuck` true))
      (if _output_get
        (set `self.ObjectifDestination` (`NavigationSystemV1.K2_GetRandomReachablePointInRadius` (`NavigationSystemV1.GetNavigationSystem`) (`self.Origin Enemy Patrol`) (`self.Range Patrol Enemy`) null null))
        (`self.Patrol`)
        (set `self.Stuck` false)))))

(event `self.ReceiveBeginPlay`
  ;[0 1 0.2663] Set Variables
  (set `CharacterMovementComponent.MaxWalkSpeed` (`self.Enemy Speed`) (`self.CharacterMovement`))
  (`SphereComponent.SetSphereRadius` (`self.Detection Player Sphere`) (`self.Detection Size`) true)
  (set `PawnSensingComponent.SightRadius` (`self.Detection Size`) (`self.PawnSensing`))
  (set `self.Origin Enemy Patrol` (`self.K2_GetActorLocation`))
  (`self.Patrol`))

(event `self.HurtBox.OnComponentBeginOverlap`
  (params (OverlappedComponent :type "PrimitiveComponent Object Reference") (OtherActor :type "Actor Object Reference") (OtherComp :type "PrimitiveComponent Object Reference") (OtherBodyIndex :type Integer) (bFromSweep :type Boolean) (SweepResult :type "HitResult Structure (by ref)"))
  ;[1 0.09183 0.06198] HP System
  (`/Engine/EditorBlueprintResources/StandardMacros.DoOnce` false :!label _label_2
    (:`Completed`
      (`KismetSystemLibrary.PrintString` "Enemy Hit")
      (`|ExecutionSequence`
        (:`then_0`
          (if (== OtherActor (`GameplayStatics.GetPlayerCharacter` 0))
            (set `self.HP` (- (`self.HP`) 1.0))
            (if (== (`self.HP`) 0.0)
              (`NiagaraFunctionLibrary.SpawnSystemAtLocation` "/Game/05_Feedbacks/Enemy/NS_EnemyKilled.NS_EnemyKilled" (`self.K2_GetActorLocation`))
              (`self.K2_DestroyActor`))))
        (:`then_1`
          (`KismetSystemLibrary.Delay` 2.0)
          (goto _label_2 :!via `Reset`))))))

(event `Patrol`
  (bind _randomlocation (`NavigationSystemV1.K2_GetRandomReachablePointInRadius` (`NavigationSystemV1.GetNavigationSystem`) (`self.Origin Enemy Patrol`) (`self.Range Patrol Enemy`) null null))
  ;[0.04179 1 0] Patrol
  (`SceneComponent.SetHiddenInGame` (`self.Widget`) true false)
  (bind (_outhit _returnvalue) (`KismetSystemLibrary.LineTraceSingle` :`Start` (`self.K2_GetActorLocation`) :`End` _randomlocation :`TraceChannel` "TraceTypeQuery1" :`DrawDebugType` "ForDuration" :`DrawTime` 3.0))
  (if (not _returnvalue)
    (bind _output_get (set `self.ObjectifDestination` _randomlocation))
    (`KismetSystemLibrary.DrawDebugLine` (`self.K2_GetActorLocation`) _output_get (struct :`R` 0.375522 :`G` 0.001665 :`B` 0.4375 :`A` 1.0) 1.0 2.0)
    (`|AIMoveTo` self _output_get null (`self.Acceptance Distance Destination`))))

(fn `DrawDetectionSphere`
  (set `self.Origin Enemy Patrol` (`self.K2_GetActorLocation`))
  (set `PawnSensingComponent.SightRadius` (`self.Detection Size`) (`self.PawnSensing`))
  (`KismetSystemLibrary.DrawDebugSphere` (`self.K2_GetActorLocation` self) (`self.Detection Size`) 12 (struct :`R` 1.0 :`G` 0.008092 :`A` 1.0) 2.0 2.0)
  (`KismetSystemLibrary.DrawDebugSphere` (`self.Origin Enemy Patrol`) (`self.Range Patrol Enemy`) 12 (struct :`G` 1.0 :`B` 1.0 :`A` 1.0) 2.0 2.0))

(fn `UserConstructionScript`
  ;[1 1 1] Debug
  (set `self.Origin Enemy Patrol` (`self.K2_GetActorLocation`))
  (set `PawnSensingComponent.SightRadius` (`self.Detection Size`) (`self.PawnSensing`))
  (`KismetSystemLibrary.DrawDebugSphere` (`self.K2_GetActorLocation` self) (`self.Detection Size`) 12 (struct :`R` 1.0 :`G` 0.008092 :`A` 1.0) 0.5 2.0)
  (`KismetSystemLibrary.DrawDebugSphere` (`self.Origin Enemy Patrol`) (`self.Range Patrol Enemy`) 12 (struct :`G` 1.0 :`B` 1.0 :`A` 1.0) 0.5 2.0))