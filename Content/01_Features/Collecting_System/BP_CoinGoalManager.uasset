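; BP_CoinGoalManager tracks coin collection in a level and fires a goal once enough coins are collected.
; On BeginPlay it finds all actors of a configurable class, uses their count as the required total and binds to the OnCollect event on each one's BP_Collectable_COMP.
; Each collect event increments a counter, and reaching the total calls HandleGoal, which currently only prints "GOAL!".
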(event `self.ReceiveBeginPlay`
  (bind _outactors (`GameplayStatics.GetAllActorsOfClass` (`self.Actor Class`)))
  ;[1 1 1] set required
  (set `self.RequiredCount` (`KismetArrayLibrary.Array_Length` _outactors))
  ;[1 1 1] listen for each coin collect
  (for _array_element _outactors
    (add `/Game/01_Features/Collecting_System/BP_Collectable_COMP.OnCollect` (`self.GetComponentByClass` _array_element "/Game/01_Features/Collecting_System/BP_Collectable_COMP.BP_Collectable_COMP_C") (delegate `OnCoinCollect`))))

(event `OnCoinCollect`
  ;[1 1 1] counter
  (bind _result (`/Engine/EditorBlueprintResources/StandardMacros.IncrementInt` (`self.Current Counter`))
    (:`  `
      (if (>= _result (`self.RequiredCount`))
        (`self.HandleGoal`)))))

(fn `HandleGoal`
  (`KismetSystemLibrary.PrintString` "GOAL!"))

(fn `UserConstructionScript`)