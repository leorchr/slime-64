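; BP_Gatherer is a collecting component that picks up actors carrying BP_Collectable when player character 0 overlaps them.
; On each pickup it broadcasts OnGathererCollect, increments Count, then calls the collectable's HandleCollect with its owner.
; OnRequiredCount fires on every increment at or above RequiredCount, not just once.
; A README graph holds unconnected example bindings for both dispatchers.
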(event `self.ReceiveBeginPlay`
  (bind _output_get (set `self.Character` (`GameplayStatics.GetPlayerCharacter` 0)))
  (add `Actor.OnActorBeginOverlap` _output_get (delegate `OnCharacterOverlap`)))

(event `OnCharacterOverlap`
  (params (OverlappedActor :type "Actor Object Reference") (OtherActor :type "Actor Object Reference"))
  (bind _returnvalue (`Actor.GetComponentByClass` OtherActor "/Game/01_Features/Collecting_System/BP_Collectable.BP_Collectable_C"))
  (`/Engine/EditorBlueprintResources/StandardMacros.IsValid` _returnvalue
    (:`Is Valid`
      (`self.OnGathererCollect` OtherActor _returnvalue)
      (`self.IncreaseCount`)
      (`/Game/01_Features/Collecting_System/BP_Collectable.HandleCollect` _returnvalue (`self.GetOwner`)))))

(event `Bind_OnRequiredCount`
  ;[1 1 1] Listen to Gathere has reached RequiredCount
  (`KismetSystemLibrary.PrintString` "Listen to Gathere has reached RequiredCount"))

(event `Bind_OnGatherCollect` :!signature `self.OnGathererCollect`
  (params (Actor :type "Actor Object Reference") (Collectable :type "/Game/01_Features/Collecting_System/BP_Collectable Object Reference"))
  ;[1 1 1] Listen to Gatherer collects Collectables
  (`KismetSystemLibrary.PrintString` " Gatherer collects Collectables"))

(fn `IncreaseCount`
  (bind _output_get (set `self.Count` (+ (`self.Count`) 1)))
  (if (>= _output_get (`self.RequiredCount`))
    (`self.OnRequiredCount`)))