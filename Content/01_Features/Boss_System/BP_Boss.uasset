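; Boss character that detects the player, then repeatedly turns to face them and charges with launch-driven dashes, sound and Niagara effects.
; DoOnce gates and delays pace each rotate-and-dash cycle, which restarts through MovementFinished.
; Hitting a wall knocks it back, tags it Stunned and rolls it over via timelines, opening a damage window.
; Player overlap with KillBox during that window removes a life, destroying the boss at zero.
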(event `self.ReceiveBeginPlay`
  (bind _returnvalue (`AddComponent|NODE_AddAudioComponent-0`))
  (set `self.Rush` _returnvalue))

(event `MovementFinished`
  (bind _rush (`self.Rush`))
  (bind (_returnvalue_roll _returnvalue_pitch _returnvalue_yaw) (`KismetMathLibrary.BreakRotator` (`KismetMathLibrary.FindLookAtRotation` (`self.K2_GetActorLocation`) (`self.K2_GetActorLocation` (`GameplayStatics.GetPlayerCharacter` 0)))))
  (`|ExecutionSequence`
    (:`then_0`
      (`KismetSystemLibrary.Delay` 2.0)
      (set `self.Can Dash?` true)
      (goto _label :!via `Reset`))
    (:`then_1`
      (goto _label_3 :!via `Reset`))
    (:`then_2`
      (`ActorComponent.Deactivate` (`self.NS_Charge`)))))

(event `self.ReceiveTick`
  (params (DeltaSeconds :type "Float (single-precision)"))
  (bind _rush (`self.Rush`))
  (bind (_returnvalue_roll _returnvalue_pitch _returnvalue_yaw) (`KismetMathLibrary.BreakRotator` (`KismetMathLibrary.FindLookAtRotation` (`self.K2_GetActorLocation`) (`self.K2_GetActorLocation` (`GameplayStatics.GetPlayerCharacter` 0)))))
  (if (`self.Player Detected?`)
    (`|ExecutionSequence`
      (:`then_0`
        ;[0.2235 0.9103 1] Character Rotates
        (`/Engine/EditorBlueprintResources/StandardMacros.DoOnce` false :!label _label
          (:`Completed`
            (set `self.PlayerPosition` (`self.K2_GetActorLocation` (`GameplayStatics.GetPlayerCharacter` 0)))
            (`self.K2_SetActorRotation` (`KismetMathLibrary.MakeRotator` _returnvalue_roll 0.0 _returnvalue_yaw)))))
      (:`then_1`
        (if (`self.Can Dash?`)
          (`SceneComponent.SetVisibility` (`self.ExclamationMark_Point`) false false :!label _label_2)
          (`SceneComponent.SetVisibility` (`self.ExclamationMark`) false false)
          ;[0.141 0.4403 1] Character Moves towards the Player
          (`self.LaunchCharacter` (* (`KismetMathLibrary.GetForwardVector` (`self.K2_GetActorRotation`)) 90.0))
          (`ActorComponent.Activate` (`self.NS_Charge`) false)
          (`ActorComponent.Activate` (`self.Dust_Movement`) false)
          (`|ExecutionSequence`
            (:`then_0`
              (`KismetSystemLibrary.Delay` (`self.DashDuration`))
              (set `self.Can Dash?` false)
              (`AudioComponent.Stop` (`self.Rush`))
              (`ActorComponent.Deactivate` (`self.NS_Charge`)))
            (:`then_1`
              (`/Engine/EditorBlueprintResources/StandardMacros.DoOnce` false :!label _label_3
                (:`Completed`
                  (`AudioComponent.SetSound` _rush null)
                  (`AudioComponent.Play` _rush 0.0))))))))))

(event `Event Force Charge`
  (goto _label_2))

(event `self.DetectionSphere.OnComponentBeginOverlap`
  (params (OverlappedComponent :type "PrimitiveComponent Object Reference") (OtherActor :type "Actor Object Reference") (OtherComp :type "PrimitiveComponent Object Reference") (OtherBodyIndex :type Integer) (bFromSweep :type Boolean) (SweepResult :type "HitResult Structure (by ref)"))
  ;[1 0.5136 0.175] Player Detection Zone
  (if (== OtherActor (`GameplayStatics.GetPlayerCharacter` 0))
    (`/Engine/EditorBlueprintResources/StandardMacros.DoOnce` false
      (:`Completed`
        (`KismetSystemLibrary.Delay` 5.0)
        (set `self.Player Detected?` true)
        (`KismetSystemLibrary.PrintString` "DEBUGGING" true true (struct :`R` 1.0 :`B` 0.837707 :`A` 1.0))))))

(event `self.CapsuleComponent.OnComponentHit`
  (params (HitComponent :type "PrimitiveComponent Object Reference") (OtherActor :type "Actor Object Reference") (OtherComp :type "PrimitiveComponent Object Reference") (NormalImpulse :type "Vector Structure") (Hit :type "HitResult Structure (by ref)"))
  (bind _ns_stun (`self.NS_Stun`))
  ;[1 0.895 0.1] Hits Something
  (if (or (`self.ActorHasTag` OtherActor "Wall") (== OtherActor (`GameplayStatics.GetPlayerCharacter` 0)))
    (`ActorComponent.Deactivate` (`self.NS_Charge`))
    (`AudioComponent.Stop` (`self.rush`))
    (set `self.Can Dash?` false)
    (if (== OtherActor (`GameplayStatics.GetPlayerPawn` 0))
      ;;[0.02631 1 0] Player Hit
      (`/Engine/EditorBlueprintResources/StandardMacros.DoOnce` false :!label _label_4
        (:`Completed`
          (`ActorComponent.Deactivate` (`self.Dust_Movement`))
          (`KismetSystemLibrary.DelayUntilNextTick`)
          (`self.Reset`)
          (`KismetSystemLibrary.Delay` 1.8)
          (`self.MovementFinished`)))
      (else
        ;;[1 0.04473 0] Enviro Hit
        (`KismetArrayLibrary.Array_Set` (`self.Tags`) 0 "Stunned")
        (`ActorComponent.Deactivate` (`self.Dust_Movement`))
        (`self.LaunchCharacter` (* (`KismetMathLibrary.NegateVector` (`KismetMathLibrary.GetForwardVector` (`self.K2_GetActorRotation`))) 3000.0))
        (bind (_direction _rotatingenemy) (`Timeline|Timeline` :`NewTime` 1.0 :!via `PlayFromStart`)
          (:`Update`
            (`self.K2_SetActorRotation` (`KismetMathLibrary.MakeRotator` _rotatingenemy))
            (set `self.CanBeDamaged?` true)
            (`ActorComponent.Activate` _ns_stun true))
          (:`Finished`
            (`KismetSystemLibrary.Delay` (`self.TimeBeforeReturn`))
            (set `self.CanBeDamaged?` false)
            (`ActorComponent.Deactivate` _ns_stun)
            (bind (_direction_2 _rotatingenemy_2) (`Timeline|Timeline_0` :!via `ReverseFromEnd`)
              (:`Update`
                (`self.K2_SetActorRotation` (`KismetMathLibrary.MakeRotator` _rotatingenemy_2))
                (`self.MovementFinished`))
              (:`Finished`
                (bind _output_get (set `self.Tags` (`self.Tags`)))
                (`KismetArrayLibrary.Array_Set` _output_get 0 "Enemy")))))))))

(event `Reset`
  ;[1 0.895 0.1] Hits Something
  ;;[0.02631 1 0] Player Hit
  (goto _label_4 :!via `Reset`))

(event `self.KillBox.OnComponentBeginOverlap`
  (params (OverlappedComponent :type "PrimitiveComponent Object Reference") (OtherActor :type "Actor Object Reference") (OtherComp :type "PrimitiveComponent Object Reference") (OtherBodyIndex :type Integer) (bFromSweep :type Boolean) (SweepResult :type "HitResult Structure (by ref)"))
  ;[0.9067 0.3036 1] Boss Death
  (`KismetSystemLibrary.PrintString` (`KismetSystemLibrary.GetDisplayName` OtherActor))
  (if (and (== OtherActor (`GameplayStatics.GetPlayerCharacter` 0)) (`self.CanBeDamaged?`))
    (set `self.BossLife` (- (`self.BossLife`) 1))
    (`self.BossLoosesHP`)
    (`ActorComponent.Activate` (`self.NS_BossDamage`) true)
    (set `self.CanBeDamaged?` false)
    (`RadialForceComponent.FireImpulse` (`self.RadialForce_Death`))
    (if (<= (`self.BossLife`) 0)
      (set `self.PlayerIsKillingEnemy?` true)
      (`ActorComponent.K2_DestroyComponent` (`self.EnemyShell`))
      (`NiagaraFunctionLibrary.SpawnSystemAtLocation` "/Game/05_Feedbacks/Enemy/NS_BossKilled.NS_BossKilled" (`self.K2_GetActorLocation`))
      (`KismetSystemLibrary.Delay` 0.2)
      (`self.K2_DestroyActor`))))

(event `self.EnemyShell.OnComponentBeginOverlap`
  (params (OverlappedComponent :type "PrimitiveComponent Object Reference") (OtherActor :type "Actor Object Reference") (OtherComp :type "PrimitiveComponent Object Reference") (OtherBodyIndex :type Integer) (bFromSweep :type Boolean) (SweepResult :type "HitResult Structure (by ref)"))
  (`KismetSystemLibrary.PrintString` "Hello"))

(fn `UserConstructionScript`)