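; Respawn component that returns the player's BP_Character to play after a game over.
; On BeginPlay it caches the player character and binds Respawn to the OnGameOver event of its BP_CharacterHealth component.
; Respawn fires game-over feedbacks, waits a configurable delay, then teleports the same character to the current checkpoint's spawn transform, or a Player Start if none is valid.
; Either path resets health.
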(event `self.ReceiveBeginPlay`
  (bind _asbp_character (cast `/Game/00_GameManager/Character/BP_Character` (`GameplayStatics.GetPlayerCharacter` 0)))
  (bind _output_get (set `self.As BP Character` _asbp_character))
  (add `CharacterHealth.OnGameOver` (`Actor.GetComponentByClass` _output_get "/Game/00_GameManager/Character/BP_CharacterHealth.BP_CharacterHealth_C") (delegate `Respawn`)))

(event `Respawn`
  (bind (_returnvalue_location _returnvalue_rotation) (`KismetMathLibrary.BreakTransform` (`Actor.GetTransform` (`GameModeBase.K2_FindPlayerStart` (`GameplayStatics.GetGameMode`) (`GameplayStatics.GetPlayerController` 0) ""))))
  (`self.OnGameOverFeedbacks`)
  (`KismetSystemLibrary.Delay` (`self.RespawnDelay`))
  (bind _currentcheckpoint (`self.CurrentCheckpoint`)
    (:`then`
      (`KismetSystemLibrary.PrintString` "Valid")
      (bind (_exactspawntransform_location _exactspawntransform_rotation) (`KismetMathLibrary.BreakTransform` (`/Game/01_Features/Respawn_System/BP_Checkpoint.ExactSpawnTransform` _currentcheckpoint)))
      (`Actor.K2_SetActorLocationAndRotation` (`self.As BP Character`) _exactspawntransform_location _exactspawntransform_rotation false false)
      (`CharacterHealth.ResetHealth` (`Actor.GetComponentByClass` (`self.As BP Character`) "/Game/00_GameManager/Character/BP_CharacterHealth.BP_CharacterHealth_C")))
    (:`else`
      (`KismetSystemLibrary.PrintString` "Not valid")
      (`Actor.K2_SetActorLocationAndRotation` (`self.As BP Character`) _returnvalue_location _returnvalue_rotation false false)
      (`CharacterHealth.ResetHealth` (`Actor.GetComponentByClass` (`self.As BP Character`) "/Game/00_GameManager/Character/BP_CharacterHealth.BP_CharacterHealth_C")))))