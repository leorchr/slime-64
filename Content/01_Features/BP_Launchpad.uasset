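; BP_Launchpad is a launch pad that flings the player character by a Strength velocity when they hit its cylinder.
; The cylinder's hit event filters for player 0, then adds Strength to their current velocity through LaunchCharacter with both overrides off.
; It also activates Niagara, deactivates the character's NSTracks effect, and triggers sound, camera shake and force feedback.
; Chained MoveComponentTo calls pop the cylinder up quickly, then ease it back down.
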(event `self.Cylinder.OnComponentHit`
  (params (HitComponent :type "PrimitiveComponent Object Reference") (OtherActor :type "Actor Object Reference") (OtherComp :type "PrimitiveComponent Object Reference") (NormalImpulse :type "Vector Structure") (Hit :type "HitResult Structure (by ref)"))
  (bind _returnvalue (`GameplayStatics.GetPlayerCharacter` 0))
  (bind _returnvalue_2 (`GameplayStatics.GetPlayerController` 0))
  (bind _cylinder (`self.Cylinder`))
  (if (== OtherActor _returnvalue)
    (`ActorComponent.Activate` (`self.Niagara`) true)
    (`ActorComponent.Deactivate` (`/Game/00_GameManager/Character/BP_Character.NS_Tracks` (cast `/Game/00_GameManager/Character/BP_Character` _returnvalue :!pure true)))
    (`Character.LaunchCharacter` _returnvalue (`self.Strength`) false false)
    (`GameplayStatics.SpawnSound2D` "/Game/04_Sounds/SFX/Launchpad/A_Launch.A_Launch" 1.0 1.0 0.0 null)
    (`PlayerController.ClientStartCameraShake` :`self` _returnvalue_2)
    (`PlayerController.K2_ClientPlayForceFeedback` _returnvalue_2 null "None" false false false)
    (`KismetSystemLibrary.MoveComponentTo` _cylinder (0.0 0.0 80.0) (struct) false false 0.1)
    (`KismetSystemLibrary.MoveComponentTo` _cylinder (0.0 0.0 0.0) (struct) false false 0.3)))

(fn `UserConstructionScript`)