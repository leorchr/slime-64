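; BP_Controller is a player controller that toggles the pause menu through its PauseMenu event.
; When the game is running, the event creates a new WBP_PauseMenu widget, stores it, adds it to the viewport, focuses it and pauses the game.
; When already paused, it removes the stored widget, restores game-only input and unpauses.
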(event `self.PauseMenu`
  (params (value :type "InputActionValue Structure (by ref)"))
  (if (not (`GameplayStatics.IsGamePaused`))
    (bind _returnvalue (`|CreateWidget` "/Game/03_UI/WBP_PauseMenu.WBP_PauseMenu_C" self))
    (bind _output_get (set `self.PauseMenuWidget` _returnvalue))
    (`UserWidget.AddToViewport` _output_get 0)
    (`Widget.SetFocus` _output_get)
    (`GameplayStatics.SetGamePaused` true)
    (else
      (`Widget.RemoveFromParent` (`self.PauseMenuWidget`))
      (`WidgetBlueprintLibrary.SetInputMode_GameOnly` self)
      (`GameplayStatics.SetGamePaused` false))))

(fn `UserConstructionScript`)