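; Character Blueprint with a Blob body that squashes and stretches when it jumps and lands.
; BeginPlay caches the Blob's base scale, limits camera pitch, enables jump apex notification and binds state-change and game-over callbacks.
; Two timelines lerp the scale toward jump and land multipliers, with a jump stopping any running land squish.
; The game-over callback sets the respawn component's delay, while the state-change handler does nothing yet.
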(event `self.ReceiveBeginPlay`
  (bind _returnvalue (`GameplayStatics.GetPlayerCameraManager` 0))
  (set `self.BaseScale` (`SceneComponent.RelativeScale3D` (`self.Blob`)))
  (add `self.OnStateChange` (delegate `OnStateChange_Event`))
  (set `PlayerCameraManager.ViewPitchMax` 20.0 _returnvalue)
  (set `PlayerCameraManager.ViewPitchMin` -80.0 _returnvalue)
  (set `CharacterMovementComponent.bNotifyApex` true (`self.CharacterMovement`))
  (add `/Game/01_Features/Respawn_System/BP_RespawnComponent.OnGameOverFeedbacks` (`self.BP_RespawnComponent`) (delegate `GameOverFeedback`)))

(event `OnStateChange_Event` :!signature `self.OnStateChange`
  (params (OldState :type "MovementState Enum" :default "Walking") (NewState :type "MovementState Enum" :default "Walking"))
  (if (`|EnumEquality` OldState "Walking")
    _))

(event `GameOverFeedback`
  (set `RespawnComponent.RespawnDelay` 10.0 (`self.BP_RespawnComponent`)) ; AS TO BE THE FIRST NODE
)

(event `JumpSqueeze`
  (bind _basescale (`self.BaseScale`))
  (bind _basescale_2 (`self.BaseScale`))
  ;[0 0.9107 1] Jump Squeeze
  (`|ExecutionSequence`
    (:`then_0`
      (bind (_direction _alpha) (`Timeline|Timeline` :!via `PlayFromStart`)
        (:`Update`
          (`SceneComponent.SetRelativeScale3D` (`self.Blob`) (`KismetMathLibrary.VLerp` _basescale_2 (* _basescale_2 (`self.JumpSqueezeStrength`)) _alpha)))))
    (:`then_1`
      ;[0 0.9107 1] Land Squish
      (bind (_direction_2 _alpha_2) (`Timeline|Timeline_0` :!via `Stop` :!label _label)
        (:`Update`
          (`SceneComponent.SetRelativeScale3D` (`self.Blob`) (`KismetMathLibrary.VLerp` _basescale (* _basescale (`self.LandSqueezeStrength`)) _alpha_2)))))))

(event `LandSquish`
  ;[0 0.9107 1] Land Squish
  (goto _label :!via `PlayFromStart`))

(event `self.OnLanded`
  (params (Hit :type "HitResult Structure (by ref)"))
  (`self.LandSquish`))

(event `self.OnJumped`
  (`self.JumpSqueeze`))

(fn `UserConstructionScript`)