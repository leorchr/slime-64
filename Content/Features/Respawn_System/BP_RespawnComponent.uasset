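; Respawn component that returns the player character to its current checkpoint after game over.
; On BeginPlay it caches player 0's BP_Character and binds Respawn to the health component's OnGameOver event.
; After RespawnDelay, it moves the character to the checkpoint's exact spawn transform and resets health.
; Without a valid checkpoint, it restarts the player at a PlayerStart through the GameMode, with no explicit health reset.
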(event `self.ReceiveBeginPlay`
  (bind _asbp_character (cast `/Game/00_GameManager/Character/BP_Character` (`GameplayStatics.GetPlayerCharacter` 0)))
  (bind _output_get (set `self.As BP Character` _asbp_character))
  (add `CharacterHealth.OnGameOver` (`Actor.GetComponentByClass` _output_get "/Game/00_GameManager/Character/BP_CharacterHealth.BP_CharacterHealth_C") (delegate `Respawn`)))

(event `Respawn`
  (bind _returnvalue (`GameplayStatics.GetGameMode`))
  (bind _currentcheckpoint (`self.CurrentCheckpoint`)
    (:`then`
      (`KismetSystemLibrary.Delay` (`self.RespawnDelay`))
      (bind (_exactspawntransform_location _exactspawntransform_rotation) (`KismetMathLibrary.BreakTransform` (`/Game/Features/Respawn_System/BP_Checkpoint.ExactSpawnTransform` _currentcheckpoint)))
      (`Actor.K2_SetActorLocationAndRotation` (`self.As BP Character`) _exactspawntransform_location _exactspawntransform_rotation false false)
      (`CharacterHealth.ResetHealth` (`Actor.GetComponentByClass` (`self.As BP Character`) "/Game/00_GameManager/Character/BP_CharacterHealth.BP_CharacterHealth_C")))
    (:`else`
      (`KismetSystemLibrary.Delay` (`self.RespawnDelay`))
      (`GameModeBase.RestartPlayerAtPlayerStart` _returnvalue null (`GameModeBase.K2_FindPlayerStart` _returnvalue (`GameplayStatics.GetPlayerController` 0) "")) ; If no Respawn Referenced, Spawn to PlayerStart
    )))