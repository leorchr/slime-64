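; BP_BossDoor is a double-leaf boss room door that opens and sends the player into another level.
; The OpenDoor event sets CanEnterBossRoom and plays a timeline that rotates both leaves around Z in opposite directions, scaled by OpenAngle.
; Once that flag is set, the player character overlapping ChangeLevelTrigger loads the soft-referenced Level, if valid.
; Nothing connected in this Blueprint calls OpenDoor.
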(event `self.ReceiveBeginPlay`)

(event `Open Door`
  (set `self.CanEnterBossRoom` true)
  (bind (_direction _newtrack_0) (`Timeline|Timeline`)
    (:`Update`
      (bind _returnvalue (* _newtrack_0 (`self.Open Angle`)))
      (`SceneComponent.K2_SetRelativeRotation` (`self.BossDoorLeaf_L`) (`KismetMathLibrary.RotatorFromAxisAndAngle` (0.0 0.0 1.0) _returnvalue) false false)
      (`SceneComponent.K2_SetRelativeRotation` (`self.BossDoorLeaf_R`) (`KismetMathLibrary.RotatorFromAxisAndAngle` (0.0 0.0 1.0) (* _returnvalue -1.0)) false false))))

(event `self.ChangeLevelTrigger.OnComponentBeginOverlap`
  (params (OverlappedComponent :type "PrimitiveComponent Object Reference") (OtherActor :type "Actor Object Reference") (OtherComp :type "PrimitiveComponent Object Reference") (OtherBodyIndex :type Integer) (bFromSweep :type Boolean) (SweepResult :type "HitResult Structure (by ref)"))
  (bind _level (`self.Level`))
  ;[1 0 0] Enter Boss Room
  (if (== (`GameplayStatics.GetPlayerCharacter` 0) OtherActor)
    (if (`self.CanEnterBossRoom`)
      (if (`KismetSystemLibrary.IsValidSoftObjectReference` _level)
        (`GameplayStatics.OpenLevelBySoftObjectPtr` _level)))))

(fn `UserConstructionScript`)