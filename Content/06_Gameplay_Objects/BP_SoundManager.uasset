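; BP_SoundManager plays the level music and nature ambiance as 2D sounds, following the player's game over and respawn.
; On BeginPlay it binds to the player's respawn and health components, then starts both sounds only if both components are valid.
; Game over fades both sounds out briefly.
; Respawn spawns both again and stores the new audio components, without stopping any still playing.
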(event `self.ReceiveBeginPlay`
  (bind _returnvalue (`GameplayStatics.GetPlayerCharacter` 0))
  (bind _returnvalue_2 (`self.GetComponentByClass` _returnvalue "/Game/01_Features/Respawn_System/BP_RespawnComponent.BP_RespawnComponent_C"))
  (bind _returnvalue_3 (`self.GetComponentByClass` _returnvalue "/Game/00_GameManager/Character/BP_CharacterHealth.BP_CharacterHealth_C"))
  (`/Engine/EditorBlueprintResources/StandardMacros.IsValid` _returnvalue_2
    (:`Is Valid`
      (add `/Game/01_Features/Respawn_System/BP_RespawnComponent.OnRespawn` _returnvalue_2 (delegate `PlayMusic`))
      (`/Engine/EditorBlueprintResources/StandardMacros.IsValid` _returnvalue_3
        (:`Is Valid`
          (add `CharacterHealth.OnGameOver` _returnvalue_3 (delegate `StopMusic`))
          (bind _returnvalue_4 (`GameplayStatics.SpawnSound2D` "/Game/04_Sounds/Music/A_MusicLevel_Cue.A_MusicLevel_Cue" 1.0 1.0 0.0 null))
          (set `self.Music` _returnvalue_4)
          (bind _returnvalue_5 (`GameplayStatics.SpawnSound2D` "/Game/04_Sounds/Ambiance/NatureSounds_Cue.NatureSounds_Cue" 1.0 1.0 0.0 null))
          (set `self.Ambiance` _returnvalue_5))))))

(event `PlayMusic`
  (bind _returnvalue (`GameplayStatics.SpawnSound2D` "/Game/04_Sounds/Music/A_MusicLevel_Cue.A_MusicLevel_Cue" 1.0 1.0 0.0 null))
  (set `self.Music` _returnvalue)
  (bind _returnvalue_2 (`GameplayStatics.SpawnSound2D` "/Game/04_Sounds/Ambiance/NatureSounds_Cue.NatureSounds_Cue" 1.0 1.0 0.0 null))
  (set `self.Ambiance` _returnvalue_2))

(event `StopMusic`
  (`AudioComponent.FadeOut` (`self.Music`) 0.4 0.0 "Linear")
  (`AudioComponent.FadeOut` (`self.Ambiance`) 0.4 0.0 "Linear"))

(fn `UserConstructionScript`)