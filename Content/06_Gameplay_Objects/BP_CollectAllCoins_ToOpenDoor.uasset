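; Collect-all objective actor for coins that opens the boss door when its inherited goal fires.
; On BeginPlay it targets BP_Coin, finds the BP_BossDoor in the level, binds OnGoal and passes the required count to the door's coin counter widget.
; Reaching the goal opens the door and blends the view to a configured camera, holds, then blends back to the previous view target.
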(event `self.ReceiveBeginPlay`
  (set `self.Actor Class` "/Game/01_Features/Collecting_System/BP_Coin.BP_Coin_C")
  (bind _returnvalue (`GameplayStatics.GetActorOfClass` "/Game/06_Gameplay_Objects/BossDoor/BP_BossDoor.BP_BossDoor_C"))
  (set `self.door` _returnvalue)
  (`parent.ReceiveBeginPlay`)
  ;[1 1 1] CHECK CAMERA
  (`/Engine/EditorBlueprintResources/StandardMacros.IsValid` (`self.Camera`)
    (:`Is Valid`
      (`/Engine/EditorBlueprintResources/StandardMacros.IsValid` (`self.door`)
        (:`Is Valid`
          (add `self.OnGoal` (delegate `OnGoal_Handler`))
          (bind _aswbp_coins_counter (cast `/Game/06_Gameplay_Objects/BossDoor/WBP_CoinsCounter` (`WidgetComponent.GetWidget` (`self.GetComponentByClass` (`self.door`) "/Script/UMG.WidgetComponent"))))
          (bind _output_get (set `self.doorWidget` _aswbp_coins_counter))
          (set `/Game/06_Gameplay_Objects/BossDoor/WBP_CoinsCounter.Required Count` (`self.RequiredCount`) _output_get))
        (:`Is Not Valid`
          (`KismetSystemLibrary.PrintString` "BP_CollectAllCoins_ToOpenDoor: CAMERA NOT FOUND" true true (struct :`R` 1.0 :`B` 0.03409 :`A` 1.0) 999999.0 :!label _label))))
    (:`Is Not Valid`
      (goto _label))))

(event `OnGoal_Handler` :!signature `self.OnGoal`
  (params (CollectAllActor :type "/Game/01_Features/Collecting_System/BP_CollectAllToGoal Object Reference"))
  ;[1 1 1] door control
  (`/Game/06_Gameplay_Objects/BossDoor/BP_BossDoor.Open Door` (`self.door`))
  ;[1 1 1] camera control
  (set `self.playerCamera` (`Controller.GetViewTarget` (`GameplayStatics.GetPlayerController` 0)))
  (`PlayerController.SetViewTargetWithBlend` (`GameplayStatics.GetPlayerController` 0) (`self.Camera`) (`self.Camera Blend Time In`) "VTBlend_EaseInOut" 2.0 false)
  (`KismetSystemLibrary.Delay` (+ (`self.Camera Blend Time In`) (`self.Camera Hold Time`)))
  (`PlayerController.SetViewTargetWithBlend` (`GameplayStatics.GetPlayerController` 0) (`self.playerCamera`) (`self.Camera Blend Time Out`) "VTBlend_EaseInOut" 2.0 false))

(fn `HandleGoal`)

(fn `UserConstructionScript`
  (`parent.UserConstructionScript`))