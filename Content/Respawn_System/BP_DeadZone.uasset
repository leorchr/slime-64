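; BP_DeadZone is a kill volume that destroys the player character and triggers a respawn when the player enters it.
; Its Box overlap acts only on player 0's character, then waits a configurable delay after destroying it.
; It then calls Respawn on the referenced BP_Respawn, or falls back to restarting the player at a PlayerStart through the GameMode when that reference is invalid.
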(event `self.Box.OnComponentBeginOverlap`
  (params (OverlappedComponent :type "PrimitiveComponent Object Reference") (OtherActor :type "Actor Object Reference") (OtherComp :type "PrimitiveComponent Object Reference") (OtherBodyIndex :type Integer) (bFromSweep :type Boolean) (SweepResult :type "HitResult Structure (by ref)"))
  (bind _returnvalue (`GameplayStatics.GetPlayerCharacter` 0))
  (bind _returnvalue_2 (`GameplayStatics.GetPlayerController` 0))
  (bind _returnvalue_3 (`GameplayStatics.GetGameMode`))
  (bind _bp_respawn (`self.BP_Respawn`))
  ;[1 1 1] Deadzone System
  (if (== OtherActor _returnvalue)
    (`self.K2_DestroyActor` _returnvalue)
    ;;[0 0.3864 0.8796] Start the Respawn System (BP_Respawn)
    (`/Engine/EditorBlueprintResources/StandardMacros.IsValid` _bp_respawn
      (:`Is Valid`
        (`KismetSystemLibrary.Delay` (`self.Delay Before Respawn`)) ; add this node to delay the respawn
        (`/Game/Respawn_System/BP_Respawn.Respawn` _bp_respawn))
      (:`Is Not Valid`
        (`KismetSystemLibrary.Delay` (`self.Delay Before Respawn`)) ; add this node to delay the respawn
        (`GameModeBase.RestartPlayerAtPlayerStart` _returnvalue_3 _returnvalue_2 (`GameModeBase.K2_FindPlayerStart` _returnvalue_3 _returnvalue_2 "")) ; If no Respawn Referenced, Spawn to PlayerStart
      ))))

(fn `UserConstructionScript`)