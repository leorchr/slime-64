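; BP_RespawnComponent is an actor component that respawns its owner after a configurable delay.
; Its Respawn event teleports the owner to the exact spawn location and rotation of the current checkpoint when one is valid.
; Without a valid checkpoint, it asks the game mode to restart the player at a player start found for player controller 0.
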(event `Respawn`
  (bind _returnvalue (`GameplayStatics.GetGameMode`))
  (bind _currentcheckpoint (`self.CurrentCheckpoint`)
    (:`then`
      (`KismetSystemLibrary.Delay` (`self.RespawnDelay`))
      (bind (_exactspawntransform_location _exactspawntransform_rotation) (`KismetMathLibrary.BreakTransform` (`/Game/Respawn_System/BP_Checkpoint.ExactSpawnTransform` _currentcheckpoint)))
      (`Actor.K2_SetActorLocationAndRotation` (`self.GetOwner`) _exactspawntransform_location _exactspawntransform_rotation false false))
    (:`else`
      (`KismetSystemLibrary.Delay` (`self.RespawnDelay`))
      (`GameModeBase.RestartPlayerAtPlayerStart` _returnvalue null (`GameModeBase.K2_FindPlayerStart` _returnvalue (`GameplayStatics.GetPlayerController` 0) "")) ; If no Respawn Referenced, Spawn to PlayerStart
    )))