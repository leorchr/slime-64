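; BP_Respawn is a checkpoint actor that spawns and possesses a new player character on respawn.
; Its trigger box stores the transform of overlapping tagged actors as CheckpointTransform, which the construction script initializes.
; The Respawn event, noted as triggered by BP_DeadZone, spawns BP_ThirdPersonCharacter for player controller 0 to possess.
; The spawn uses this actor's own location and rotation, taking only scale from CheckpointTransform.
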(event `self.ReceiveBeginPlay`)

(event `self.TriggerBox.OnComponentBeginOverlap`
  (params (OverlappedComponent :type "PrimitiveComponent Object Reference") (OtherActor :type "Actor Object Reference") (OtherComp :type "PrimitiveComponent Object Reference") (OtherBodyIndex :type Integer) (bFromSweep :type Boolean) (SweepResult :type "HitResult Structure (by ref)"))
  ;[1 1 1] Respawn System
  ;;[0.9734 0.1683 0.000304] Set Checkpoint When Overlapping With Actor
  (if (`self.ActorHasTag` OtherActor (`self.Tag`))
    (set `self.Checkpoint Transform` (`self.GetTransform` OtherActor))))

(event `Respawn`
  (bind (_returnvalue_location _returnvalue_rotation) (`KismetMathLibrary.BreakTransform` (`self.GetTransform`)))
  (bind (_checkpoint_transform_location _checkpoint_transform_rotation _checkpoint_transform_scale) (`KismetMathLibrary.BreakTransform` (`self.Checkpoint Transform`)))
  ;[1 1 1] Respawn System
  ;;[0.9301 0.03689 0.03689] Respawn Event (Triggered by BP_DeadZone)
  ;;;[0.000304 0.3712 0.8469] Reference in "Class" the Actor you want to respawn
  (bind _returnvalue (`|SpawnActorFromClass` "/Game/ThirdPerson/Blueprints/BP_ThirdPersonCharacter.BP_ThirdPersonCharacter_C" (`KismetMathLibrary.MakeTransform` _returnvalue_location _returnvalue_rotation _checkpoint_transform_scale) "Undefined" "MultiplyWithRoot" null null))
  (`Controller.Possess` (`GameplayStatics.GetPlayerController` 0) _returnvalue))

(fn `UserConstructionScript`
  (set `self.Checkpoint Transform` (`self.GetTransform` (`self.Target`))))